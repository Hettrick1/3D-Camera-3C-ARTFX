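; BP_TP is a teleporter actor that moves a player to the Arrow location of its linked NextTp teleporter.
; TeleportPlayer, with no caller in this file, passes a DoOnce and sets the player's location without sweep.
; The DoOnce resets right after a successful move, but stays closed if NextTp is invalid.
; The Box is made visible by the Construction Script and hidden at BeginPlay.
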(event `self.ReceiveBeginPlay`
  (`SceneComponent.SetHiddenInGame` (`self.Box`) true true))

(event `/Game/Camera-3C/Blueprints/2D/BPI/BPI_TP.TeleportPlayer`
  (params (playerRef :type "/Game/Camera-3C/Blueprints/2D/BP_StardewValleyPlayer Object Reference"))
  (bind _nexttp (`self.NextTp`))
  (`/Engine/EditorBlueprintResources/StandardMacros.DoOnce` false :!label _label
    (:`Completed`
      (`/Engine/EditorBlueprintResources/StandardMacros.IsValid` _nexttp
        (:`Is Valid`
          (`self.K2_SetActorLocation` playerRef (`SceneComponent.K2_GetComponentLocation` (`/Game/Camera-3C/Blueprints/2D/MAP_BP/BP_TP.Arrow` _nexttp)) false true)
          (`self.ResetDoOnceTP`))))))

(event `ResetDoOnceTP`
  (goto _label :!via `Reset`))

(fn `UserConstructionScript`
  (`SceneComponent.SetHiddenInGame` (`self.Box`) false true))